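; Player interaction component for the first-person character, handling item pickup, dropping and belt-slot switching.
; A self-repeating delayed sphere trace from the camera tracks the BPI_Item in view, which E attaches to the hand and Q drops, updating the belt inventory and widget.
; Keys 1–3 and active-slot updates destroy and respawn the held actor from slot data.
; A separate line trace flags doors, though left-click only prints a debug message.
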(event Custom|Looking
  (bind _first_person_camera (Variables|Default|GetFirst%20Person%20Camera))
  (bind _returnvalue (Transformation|GetWorldLocation _first_person_camera))
  ;[0.15 0.15 0.15 0.5] Pick up last touched item - Looking
  (Utilities|FlowControl|Delay 0.2)
  (bind (_outhit _returnvalue_2) (Collision|SphereTraceByChannel _returnvalue (+ _returnvalue (* (Math|Vector|GetForwardVector _first_person_camera) (Variables|Default|GetLookDistance))) 5e+01 "TraceTypeQuery1" false 0 "None" true "(R=1.000000,G=0.000000,B=0.000000,A=1.000000)" "(R=0.000000,G=1.000000,B=0.000000,A=1.000000)" 1.0))
  (if _returnvalue_2
    (if (Utilities|DoesObjectImplementInterface (.HitActor (Collision|BreakHitResult _outhit)) "/Game/BlueprintInventory/Inventory/Prep/BPI_Item.BPI_Item_C")
      (Variables|Default|SetLast%20Touched%20Item (.HitActor (Collision|BreakHitResult _outhit)))
      (Development|PrintText (Utilities|Text|FormatText "Press E to pickup {name}" (Utilities|GetDisplayName (.HitActor (Collision|BreakHitResult _outhit)))))
      (else
        (Variables|Default|SetLast%20Touched%20Item 0)))
    (else
      (Variables|Default|SetLast%20Touched%20Item 0)))
  (CallFunction|Looking))

(event Custom|Try%20to%20Pick%20Up
  (bind _player (Variables|Default|GetPlayer))
  ;[0.15 0.15 0.15 0.5] Try to Pick Up function
  (Variables|Default|GetHeldItem
    (:then
      _)
    (:else
      _))
  (bind _last_touched_item (Variables|Default|GetLast%20Touched%20Item)
    (:then
      (bind _item_type (Class|BPIItem|Pickup(Message) _last_touched_item self))
      (Transformation|AttachComponentToComponent _last_touched_item (Variables|/Game/BP_FirstPersonCharacter.BP_FirstPersonCharacter_C|GetHandHeldPoint (Variables|Default|GetPlayer)) "None" "KeepRelative" "KeepRelative" "KeepRelative" true)
      (Variables|Default|SetHeldItem _last_touched_item)
      (Default|SetSlot (Variables|/Game/BP_FirstPersonCharacter.BP_FirstPersonCharacter_C|GetBPC_BeltInv _player) _item_type (Variables|Default|GetActive%20Slot))
      (Default|RefreshGrid (Variables|/Game/BlueprintInventory/Inventory/W_Belt.W_Belt_C|GetW_InventoryGrid (Variables|/Game/BP_FirstPersonCharacter.BP_FirstPersonCharacter_C|GetBelt%20Widget _player))))
    (:else
      (Development|PrintText "We are not looking at anything"))))

(event Custom|Try%20to%20Interact
  (bind _first_person_camera (Variables|Default|GetFirst%20Person%20Camera))
  (bind _returnvalue (Transformation|GetWorldLocation _first_person_camera))
  ;[0.15 0.15 0.15 0.5] Try to Interact Code
  (bind (_outhit _returnvalue_2) (Collision|LineTraceByChannel _returnvalue (+ _returnvalue (* (Math|Vector|GetForwardVector _first_person_camera) (Variables|Default|GetLookDistance))) "TraceTypeQuery1" true (Utilities|Array|MakeArray (Game|GetPlayerCharacter 0) 0) "Persistent"))
  (if _returnvalue_2
    (Development|PrintText (Utilities|Text|FormatText "I am touching {name} with my eyes" (Utilities|GetDisplayName (.HitActor (Collision|BreakHitResult _outhit)))))
    (Rendering|Decal|SpawnDecalatLocation 0 "0, 0, 0" (.Location (Collision|BreakHitResult _outhit)) "-90.000000,0.000000,0.000000" 0.0)
    (Utilities|Casting|CastToBP_Door (.HitActor (Collision|BreakHitResult _outhit))
      (:then
        (Variables|Default|SetCanOpenDoor true))
      (:CastFailed
        (Variables|Default|SetCanOpenDoor false)))
    (CallFunction|TrytoInteract)
    (else
      (Variables|Default|SetCanOpenDoor false)
      (CallFunction|TrytoInteract))))

(event Custom|Try%20to%20Use
  ;[0.15 0.15 0.15 0.5] Try to Use
  (bind _helditem (Variables|Default|GetHeldItem)
    (:then
      (Class|BPIItem|Use(Message) _helditem))
    (:else
      (Development|PrintText "We aren't holding anything"))))

(event Custom|Try%20to%20Drop
  (bind _player (Variables|Default|GetPlayer))
  ;[0.15 0.15 0.15 0.5] Try to Drop
  (bind _helditem (Variables|Default|GetHeldItem)
    (:then
      (Transformation|DetachFromActor (Variables|Default|GetHeldItem) "KeepRelative" "KeepRelative" "KeepRelative")
      (Class|BPIItem|Drop(Message) _helditem)
      (Default|SetSlot (Variables|/Game/BP_FirstPersonCharacter.BP_FirstPersonCharacter_C|GetBPC_BeltInv _player) "NewEnumerator8" (Variables|Default|GetActive%20Slot))
      (Default|RefreshGrid (Variables|/Game/BlueprintInventory/Inventory/W_Belt.W_Belt_C|GetW_InventoryGrid (Variables|/Game/BP_FirstPersonCharacter.BP_FirstPersonCharacter_C|GetBelt%20Widget _player))))
    (:else
      ;[0.15 0.15 0.15 0.5] Try to Use
      (Development|PrintText "We aren't holding anything"))))

(event Custom|Swap%20Active%20Item
  (params (New%20Slot%20Index :type Integer))
  (bind _player (Variables|Default|GetPlayer))
  (bind _handheldpoint (Variables|/Game/BP_FirstPersonCharacter.BP_FirstPersonCharacter_C|GetHandHeldPoint _player))
  ;[0.15 0.15 0.15 0.5] Swap Active Item
  (if (!= (Variables|Default|GetActive%20Slot) New%20Slot%20Index)
    (bind _output_get (Variables|Default|SetActive%20Slot New%20Slot%20Index))
    (bind _helditem (Variables|Default|GetHeldItem)
      (:then
        (Actor|DestroyActor _helditem))
      (:else
        _))
    (if (Utilities|Enum|NotEqual(Enum) (.Enum (Utilities|Struct|BreakS_Item (Default|GetSlot (Variables|/Game/BP_FirstPersonCharacter.BP_FirstPersonCharacter_C|GetBPC_BeltInv (Variables|Default|GetPlayer)) _output_get))) "NewEnumerator8")
      (bind _returnvalue (Game|SpawnActorfromClass (.ActorBP (Utilities|Struct|BreakS_Item (Default|GetSlot (Variables|/Game/BP_FirstPersonCharacter.BP_FirstPersonCharacter_C|GetBPC_BeltInv (Variables|Default|GetPlayer)) _output_get))) (Transformation|GetRelativeTransform _handheldpoint) "Undefined" "MultiplyWithRoot" 0 0))
      (bind _output_get_2 (Variables|Default|SetHeldItem _returnvalue))
      (Class|BPIItem|Pickup(Message) _output_get_2 self)
      (Transformation|AttachComponentToComponent _output_get_2 _handheldpoint "None" "SnapToTarget" "SnapToTarget" "KeepRelative" true)
      (else
        (Development|PrintText "Swapping to an empty slot")
        (Actor|DestroyActor (Variables|Default|GetHeldItem))
        (Variables|Default|SetHeldItem 0)))
    (else
      (Development|PrintText "Swapping to same slot, ignore"))))

(event Custom|OnSlotUpdated_Event
  (params (Updated%20Slot%20Index :type Integer))
  ;[0.15 0.15 0.15 0.5] Cast to First Person from Event Play
  (CallFunction|UpdateHeldItem Updated%20Slot%20Index))

(event Custom|Update%20Held%20Item
  (params (Newly%20Changed%20Slot :type Integer))
  (bind _player (Variables|Default|GetPlayer))
  (bind _handheldpoint (Variables|/Game/BP_FirstPersonCharacter.BP_FirstPersonCharacter_C|GetHandHeldPoint _player))
  (if (== (Variables|Default|GetActive%20Slot) Newly%20Changed%20Slot)
    ;[0.15 0.15 0.15 0.5] Swap Active Item
    (bind _helditem (Variables|Default|GetHeldItem)
      (:then
        (Actor|DestroyActor _helditem))
      (:else
        _))
    (if (Utilities|Enum|NotEqual(Enum) (.Enum (Utilities|Struct|BreakS_Item (Default|GetSlot (Variables|/Game/BP_FirstPersonCharacter.BP_FirstPersonCharacter_C|GetBPC_BeltInv (Variables|Default|GetPlayer)) (stale Custom|Swap%20Active%20Item _output_get)))) "NewEnumerator8")
      (bind _returnvalue (Game|SpawnActorfromClass (.ActorBP (Utilities|Struct|BreakS_Item (Default|GetSlot (Variables|/Game/BP_FirstPersonCharacter.BP_FirstPersonCharacter_C|GetBPC_BeltInv (Variables|Default|GetPlayer)) (stale Custom|Swap%20Active%20Item _output_get)))) (Transformation|GetRelativeTransform _handheldpoint) "Undefined" "MultiplyWithRoot" 0 0))
      (bind _output_get (Variables|Default|SetHeldItem _returnvalue))
      (Class|BPIItem|Pickup(Message) _output_get self)
      (Transformation|AttachComponentToComponent _output_get _handheldpoint "None" "SnapToTarget" "SnapToTarget" "KeepRelative" true)
      (else
        (Development|PrintText "Swapping to an empty slot")
        (Actor|DestroyActor (Variables|Default|GetHeldItem))
        (Variables|Default|SetHeldItem 0)))))

(event EventBeginPlay
  ;[0.15 0.15 0.15 0.5] Cast to First Person from Event Play
  (bind _asbp_first_person_character (Utilities|Casting|CastToBP_FirstPersonCharacter (Components|GetOwner)))
  (Variables|Default|SetPlayer _asbp_first_person_character)
  (Variables|Default|SetFirst%20Person%20Camera (Variables|/Game/BP_FirstPersonCharacter.BP_FirstPersonCharacter_C|GetFirstPersonCamera _asbp_first_person_character))
  (CallFunction|Looking)
  (CallFunction|SwapActiveItem)
  (EventDispatchers|AssignOnSlotUpdated (Variables|/Game/BP_FirstPersonCharacter.BP_FirstPersonCharacter_C|GetBPC_BeltInv (Variables|Default|GetPlayer)) (delegate Custom|OnSlotUpdated_Event)))

(event Input|KeyboardEvents|Q
  (params (Key :type Key%20Structure :default "None"))
  ;[0.15 0.15 0.15 0.5] Q button - Drop
  (:Pressed
    (CallFunction|TrytoDrop)))

(event Input|KeyboardEvents|E
  (params (Key :type Key%20Structure :default "None"))
  ;[0.15 0.15 0.15 0.5] E key input
  (:Pressed
    (CallFunction|TrytoPickUp)))

(event Input|MouseEvents|LeftMouseButton
  (params (Key :type Key%20Structure :default "None"))
  ;[0.15 0.15 0.15 0.5] Left MB Click to check to open door
  (:Pressed
    (if (Variables|Default|GetCanOpenDoor)
      (Development|PrintString "Destroy door"))))

(event Input|MouseEvents|RightMouseButton
  (params (Key :type Key%20Structure :default "None"))
  ;[0.15 0.15 0.15 0.5] Looking - RMB
  (:Pressed
    (Development|PrintString "Hello")
    (CallFunction|Looking)))

(event Input|KeyboardEvents|1
  (params (Key :type Key%20Structure :default "None"))
  ;[0.15 0.15 0.15 0.5] 1, 2, and 3 interchanges
  (:Pressed
    (CallFunction|SwapActiveItem)))

(event Input|KeyboardEvents|2
  (params (Key :type Key%20Structure :default "None"))
  ;[0.15 0.15 0.15 0.5] 1, 2, and 3 interchanges
  (:Pressed
    (CallFunction|SwapActiveItem 1)))

(event Input|KeyboardEvents|3
  (params (Key :type Key%20Structure :default "None"))
  ;[0.15 0.15 0.15 0.5] 1, 2, and 3 interchanges
  (:Pressed
    (CallFunction|SwapActiveItem 2)))