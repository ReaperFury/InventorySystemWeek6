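; Inventory component that stores items as an array of enums, one per slot.
; GetSlot resolves a slot's enum to its details through GetItemDetails, which loops over every DT_Items row until the Enum field matches.
; SetSlot writes one slot and calls OnSlotUpdated with its index, while SetEnumArray replaces the whole array and calls OnRefreshGrid.
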(event EventBeginPlay)

(event EventTick
  (params (DeltaSeconds :type Float%20%28single-precision%29)))

(fn GetItemDetails
  (params (RequestedItem :type E_Item%20Enum :default "NewEnumerator0"))
  (bind _outrownames (DataTable|GetDataTableRowNames "/Game/BlueprintInventory/DataTables/DT_Items.DT_Items"))
  (for _array_element _outrownames
    (bind _returnvalue (Utilities|GetDataTableRow "/Game/BlueprintInventory/DataTables/DT_Items.DT_Items" _array_element)
      (:then
        (if (Utilities|Enum|Equal(Enum) (.Enum (Utilities|Struct|BreakS_Item _returnvalue)) RequestedItem)
          (return _returnvalue))))))

(fn GetSlot
  (params (Requested%20Slot :type Integer))
  ;[0.15 0.15 0.15 0.5] Get Slot Details
  (bind _itemdetails (CallFunction|GetItemDetails (Utilities|Array|Get(acopy) (Variables|Default|GetEnumInventory) Requested%20Slot)))
  (return _itemdetails))

(fn SetSlot
  (params (Item :type E_Item%20Enum :default "NewEnumerator8") (Slot%20Index :type Integer))
  (Utilities|Array|SetArrayElem (Variables|Default|GetEnumInventory) Slot%20Index Item)
  (Default|CallOnSlotUpdated Slot%20Index))

(fn SetEnumArray
  (params (EnumInventory :type Array%20of%20E_Item%20Enums :default "NewEnumerator8"))
  (Variables|Default|SetEnumInventory EnumInventory)
  (Default|CallOnRefreshGrid))