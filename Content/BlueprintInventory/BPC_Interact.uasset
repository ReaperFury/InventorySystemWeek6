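; Interaction component for the first-person character that detects items in view and lets the player trigger their pickup message.
; Left click starts a self-repeating delayed sphere trace from the owner's camera, with debug drawing.
; Hit actors implementing BPI_Item are cached as the last touched item and prompt on screen.
; Pressing E calls PickupMessage on that item; an older line-trace version remains unconnected.
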(event Custom|Looking
  (bind _first_person_camera (Variables|Default|GetFirst%20Person%20Camera))
  (bind _returnvalue (Transformation|GetWorldLocation _first_person_camera))
  ;[0.15 0.15 0.15 0.5] Pick up last touched item
  (Utilities|FlowControl|Delay 0.2)
  (bind (_outhit _returnvalue_2) (Collision|SphereTraceByChannel _returnvalue (+ _returnvalue (* (Math|Vector|GetForwardVector _first_person_camera) (Variables|Default|GetLookDistance))) 5e+01 "TraceTypeQuery1" false 0 "ForDuration" true "(R=1.000000,G=0.000000,B=0.000000,A=1.000000)" "(R=0.000000,G=1.000000,B=0.000000,A=1.000000)" 1.0))
  (if _returnvalue_2
    (if (Utilities|DoesObjectImplementInterface (.HitActor (Collision|BreakHitResult _outhit)) "/Game/BlueprintInventory/BPI_Item.BPI_Item_C")
      (Variables|Default|SetLast%20Touched%20Item (.HitActor (Collision|BreakHitResult _outhit)))
      (Development|PrintText (Utilities|Text|FormatText "Press E to pickup {name}" (Utilities|GetDisplayName (.HitActor (Collision|BreakHitResult _outhit)))))
      (else
        (Variables|Default|SetLast%20Touched%20Item 0))))
  (CallFunction|Looking))

(event Custom|Try%20to%20Pick%20Up
  (bind _last_touched_item (Variables|Default|GetLast%20Touched%20Item)
    (:then
      (Class|BPIItem|Pickup(Message) _last_touched_item))
    (:else
      (Development|PrintText "We're not looking at anything. "))))

(event EventBeginPlay
  (bind _asbp_first_person_character (Utilities|Casting|CastToBP_FirstPersonCharacter (Components|GetOwner)))
  (Variables|Default|SetFirst%20Person%20Camera (Variables|/Game/BP_FirstPersonCharacter.BP_FirstPersonCharacter_C|GetFirstPersonCamera _asbp_first_person_character)))

(event EventTick
  (params (DeltaSeconds :type Float%20%28single-precision%29)))

(event Input|MouseEvents|LeftMouseButton
  (params (Key :type Key%20Structure :default "None"))
  ;[0.15 0.15 0.15 0.5] Pick up last touched item
  (:Pressed
    (Development|PrintString "Hello")
    (CallFunction|Looking)))

(event Input|KeyboardEvents|E
  (params (Key :type Key%20Structure :default "None"))
  (:Pressed
    (CallFunction|TrytoPickUp)))