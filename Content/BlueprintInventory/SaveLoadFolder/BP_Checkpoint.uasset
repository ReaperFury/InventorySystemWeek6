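; BP_Checkpoint is an overlap-triggered checkpoint actor that saves the player's progress.
; On BeginPlay it casts and caches the GM_Saveload game mode.
; When BP_FirstPersonCharacter overlaps it, it passes the belt and backpack inventories, transform and forward vector to the game mode's Save, then prints an activation message.
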(event EventBeginPlay
  (bind _asgm_saveload (Utilities|Casting|CastToGM_Saveload (Game|GetGameMode)))
  (Variables|Default|SetGame%20Mode _asgm_saveload))

(event Collision|EventActorBeginOverlap
  (params (OtherActor :type Actor%20Object%20Reference))
  (bind _asbp_first_person_character (Utilities|Casting|CastToBP_FirstPersonCharacter OtherActor))
  (Default|Save (Variables|Default|GetGame%20Mode) (Variables|/Game/BlueprintInventory/Inventory/BPC_Inventory.BPC_Inventory_C|GetEnumInventory (Variables|/Game/BP_FirstPersonCharacter.BP_FirstPersonCharacter_C|GetBPC_BeltInv _asbp_first_person_character)) (Variables|/Game/BlueprintInventory/Inventory/BPC_Inventory.BPC_Inventory_C|GetEnumInventory (Variables|/Game/BP_FirstPersonCharacter.BP_FirstPersonCharacter_C|GetBPC_BackpackInv _asbp_first_person_character)) (Transformation|GetActorTransform _asbp_first_person_character) (Transformation|GetActorForwardVector _asbp_first_person_character))
  (Development|PrintString "Checkpoint Activated"))

(fn ConstructionScript)