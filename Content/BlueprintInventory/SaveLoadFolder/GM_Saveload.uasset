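; GM_Saveload is a save/load Blueprint for player inventories and per-level state, using SG_Player and SG_LevelState save objects.
; BeginPlay loads existing saves or creates new objects, but its slot names differ from those Load reads.
; Load activates level actors, then restores the character's belt, backpack and transform.
; Save writes only belt and backpack; its level-state branch is disconnected, and Pickup is empty.
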(event EventBeginPlay
  (Development|PrintString "Player Load")
  (Utilities|FlowControl|Sequence
    (:then_0
      (bind _returnvalue (SaveGame|DoesSaveGameExist))
      (if _returnvalue
        (Utilities|FlowControl|Delay 0.2)
        (CallFunction|Load)
        (else
          (bind _returnvalue_2 (SaveGame|CreateSaveGameObject "/Game/BlueprintInventory/SaveLoadFolder/SG_Player.SG_Player_C"))
          (Variables|Default|SetPlayer%20Save _returnvalue_2))))
    (:then_1
      (bind _returnvalue_3 (Game|GetCurrentLevelName true))
      (bind _returnvalue_4 (SaveGame|DoesSaveGameExist (Utilities|String|Append _returnvalue_3 (Variables|Default|GetSlot%20Name))))
      (if _returnvalue_4
        (CallFunction|Load)
        (else
          (bind _returnvalue_5 (SaveGame|CreateSaveGameObject "/Game/BlueprintInventory/SaveLoadFolder/SG_LevelState.SG_LevelState_C"))
          (Variables|Default|SetLevelState _returnvalue_5))))))

(fn ConstructionScript)

(fn Save
  (params (Belt :type Array%20of%20E_Item%20Enums :default "NewEnumerator8") (PlayerInv :type Array%20of%20E_Item%20Enums :default "NewEnumerator8") (Location :type Transform) (Forward :type Vector))
  (bind _player_save (Variables|Default|GetPlayer%20Save))
  ;[0.15 0.15 0.15 0.5] Save Function
  (Utilities|FlowControl|Sequence
    (:then_0
      (Variables|/Game/BlueprintInventory/SaveLoadFolder/SG_Player.SG_Player_C|SetBelt _player_save Belt)
      (Variables|/Game/BlueprintInventory/SaveLoadFolder/SG_Player.SG_Player_C|SetPlayerInv _player_save PlayerInv)
      (SaveGame|SaveGametoSlot (Variables|Default|GetPlayer%20Save) (Variables|Default|GetSlot%20Name)))))

(fn Load
  ;[0.15 0.15 0.15 0.5] Load Function
  (Utilities|FlowControl|Sequence
    (:then_0
      (bind _returnvalue (SaveGame|LoadGamefromSlot (Variables|Default|GetSlot%20Name)))
      (bind _assg_player (Utilities|Casting|CastToSG_Player _returnvalue))
      (Variables|Default|SetPlayer%20Save _assg_player))
    (:then_1
      (bind _returnvalue_2 (Game|GetCurrentLevelName true))
      (bind _returnvalue_3 (SaveGame|LoadGamefromSlot (Utilities|String|Append _returnvalue_2 "_" (Variables|Default|GetSlot%20Name))))
      (bind _assg_level_state (Utilities|Casting|CastToSG_LevelState _returnvalue_3))
      (bind _output_get (Variables|Default|SetLevelState _assg_level_state))
      (Default|ActivateActors _output_get)
      (bind _asbp_first_person_character (Utilities|Casting|CastToBP_FirstPersonCharacter (Game|GetPlayerCharacter 0)))
      (Default|SetEnumArray (Variables|/Game/BP_FirstPersonCharacter.BP_FirstPersonCharacter_C|GetBPC_BeltInv _asbp_first_person_character) (Variables|/Game/BlueprintInventory/SaveLoadFolder/SG_Player.SG_Player_C|GetBelt (Variables|Default|GetPlayer%20Save)))
      (Default|SetEnumArray (Variables|/Game/BP_FirstPersonCharacter.BP_FirstPersonCharacter_C|GetBPC_BackpackInv _asbp_first_person_character) (Variables|/Game/BlueprintInventory/SaveLoadFolder/SG_Player.SG_Player_C|GetPlayerInv (Variables|Default|GetPlayer%20Save)))
      (Default|LoadTransform _asbp_first_person_character (Variables|/Game/BlueprintInventory/SaveLoadFolder/SG_Player.SG_Player_C|GetLocation (Variables|Default|GetPlayer%20Save)) (Variables|/Game/BlueprintInventory/SaveLoadFolder/SG_Player.SG_Player_C|GetForward (Variables|Default|GetPlayer%20Save)))
      (Pawn|SetControlRotation (Game|GetPlayerController 0) (.Rotation (Math|Transform|BreakTransform (Variables|/Game/BlueprintInventory/SaveLoadFolder/SG_Player.SG_Player_C|GetLocation (Variables|Default|GetPlayer%20Save)))))
      (Development|PrintText "Inventory Updated")
      (return))))

(fn Pickup)