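; Stats component that holds a struct of health, mana, stamina, gold, experience and a saved location for its owner.
; GetCanSprint gates sprinting on remaining stamina, and Sprinting rebuilds the struct with stamina reduced by a given amount, without clamping.
; Tick prints health, mana, stamina and experience on screen as debug text, using the frame's delta time as the display duration.
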(event Custom|Debug%20Stats
  (params (Duration :type Float%20%28double-precision%29))
  (bind _stats (Variables|Default|GetStats))
  (bind (_health _mana _stamina _savedlocation _gold _experience) (Utilities|Struct|BreakS_Stats _stats))
  (Development|PrintText (Utilities|Text|FormatText "HP: {health}, MP: {mana}, Stam: {stamina}, XP: {experience}" _health _mana _stamina _experience) true true (Utilities|Struct|MakeLinearColor 1.0 0.0 0.1 1.0) Duration))

(event EventBeginPlay)

(event EventTick
  (params (DeltaSeconds :type Float%20%28single-precision%29))
  (CallFunction|DebugStats DeltaSeconds))

(fn GetCanSprint
  (return (> (.stamina (Variables|Default|GetStats)) 1.0)))

(fn Sprinting
  (params (Reduce%20Stamina%20By :type Float%20%28double-precision%29))
  (Variables|Default|SetStats (Utilities|Struct|MakeS_Stats (.health (Variables|Default|GetStats)) (.mana (Variables|Default|GetStats)) (- (.stamina (Variables|Default|GetStats)) Reduce%20Stamina%20By) (.savedlocation (Variables|Default|GetStats)) (.gold (Variables|Default|GetStats)) (.experience (Variables|Default|GetStats)))))