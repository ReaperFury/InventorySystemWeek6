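; BP_Key is a holdable key item that removes a door when used, consuming itself.
; Pickup stores the owner, disables mesh collision and returns the item type; Drop clears the owner's held item and restores collision.
; Use runs a debug-drawn visibility line trace from the mesh, destroying key and BP_Door on a hit.
; The trace end omits the mesh location, so it lands near world origin.
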(event Custom|Pickup_1_1
  (params (Owner :type Actor%20Object%20Reference))
  (Collision|SetCollisionEnabled (Variables|Default|GetKey%20Mesh) "NoCollision"))

(event EventAlternateUse)

(event EventUse
  (bind _key_mesh (Variables|Default|GetKey%20Mesh))
  (bind _returnvalue (Math|Vector|GetForwardVector _key_mesh))
  (bind _outhit (Collision|LineTraceByChannel (Transformation|GetWorldLocation _key_mesh) (+ _returnvalue (* _returnvalue 3e+02)) "TraceTypeQuery1" false 0 "ForDuration"))
  (bind _asbp_door (Utilities|Casting|CastToBP_Door (.HitActor (Collision|BreakHitResult _outhit))))
  (Actor|DestroyActor self))

(event EventDrop
  (Variables|/Game/BlueprintInventory/Prep/BPC_Interact.BPC_Interact_C|SetHeldItem (Variables|Default|GetOwner_0) 0)
  (Collision|SetCollisionEnabled (Variables|Default|GetKey%20Mesh) "QueryAndPhysics"))

(fn ConstructionScript)

(fn Pickup
  (params (Owner :type BPC%20Interact%20Object%20Reference))
  (Variables|Default|SetOwner_0 Owner)
  (Collision|SetCollisionEnabled (Variables|Default|GetKey%20Mesh) "NoCollision")
  (return (Variables|Default|GetItem%20Type)))