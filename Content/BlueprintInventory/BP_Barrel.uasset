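; BP_Barrel is a barrel with an inventory whose lid hinge swings open when the first-person character overlaps its sphere.
; A timeline lerps the hinge's roll, playing or reversing by a Reverse flag.
; Both begin and end overlap pass false, so nothing here triggers closing.
; When the timeline finishes with Reverse false, it prints debug text naming the first inventory item.
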(event OnComponentBeginOverlap(Sphere)
  (params (OverlappedComponent :type Primitive%20Component%20Object%20Reference) (OtherActor :type Actor%20Object%20Reference) (OtherComp :type Primitive%20Component%20Object%20Reference) (OtherBodyIndex :type Integer) (bFromSweep :type Boolean) (SweepResult :type Hit%20Result%20Structure%20%28by%20ref%29))
  ;[0.15 0.15 0.15 0.5] Player comes in contact with barrel
  (Utilities|Casting|CastToBP_FirstPersonCharacter OtherActor)
  (CallFunction|OpenBarrel false))

(event OnComponentEndOverlap(Sphere)
  (params (OverlappedComponent :type Primitive%20Component%20Object%20Reference) (OtherActor :type Actor%20Object%20Reference) (OtherComp :type Primitive%20Component%20Object%20Reference) (OtherBodyIndex :type Integer))
  (Utilities|Casting|CastToBP_FirstPersonCharacter OtherActor)
  (CallFunction|OpenBarrel false))

(event Custom|open%20barrel
  (params (Reverse :type Boolean))
  (if Reverse
    (bind _newtrack_0 (Timeline|Open%20timeline Reverse)
      (:Update
        (Transformation|SetRelativeRotation (Variables|Default|Gethinge) (Math|Rotator|MakeRotator (Math|Float|Lerp 0.0 6e+01 _newtrack_0) 0.0 0.0) false false))
      (:Finished
        (if (not Reverse)
          (Development|PrintText "Opening barrel")
          (Development|PrintText (Utilities|Text|FormatText "First item in barrel is {name}." (.Name (Utilities|Struct|BreakS_Item (Utilities|Array|Get(acopy) (Variables|Default|GetInventory))))) true true "(R=0.000000,G=0.660000,B=1.000000,A=1.000000)" 2e+01))))
    (else
      (Timeline|Open%20timeline Play))))

(fn ConstructionScript)